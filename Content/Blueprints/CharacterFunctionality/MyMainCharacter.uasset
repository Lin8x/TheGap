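; MyMainCharacter is a first-person character Blueprint with an early, debug-stage Interact input.
; Pressing Interact runs a multi line trace against WorldStatic objects from the camera, drawn for debugging.
; The trace direction combines the camera's relative pitch and roll with the capsule's world yaw.
; The hit results are unused, and debug messages print on every press through an always-true branch.
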(event `InputAction|Interact`
  (params (Key :type "Key Structure"))
  (bind _firstpersoncamera (`self.FirstPersonCamera`))
  (bind _returnvalue (`SceneComponent.K2_GetComponentLocation` _firstpersoncamera))
  (bind (_returnvalue_roll _returnvalue_pitch _returnvalue_yaw) (`KismetMathLibrary.BreakRotator` (`SceneComponent.K2_GetComponentRotation` (`self.CapsuleComponent`))))
  (bind (_relativerotation_roll _relativerotation_pitch) (`KismetMathLibrary.BreakRotator` (`SceneComponent.RelativeRotation` _firstpersoncamera)))
  (:`Pressed`
    (`KismetSystemLibrary.LineTraceMultiForObjects` :`Start` _returnvalue :`End` (+ _returnvalue (* (`KismetMathLibrary.GetForwardVector` (`KismetMathLibrary.MakeRotator` _relativerotation_roll _relativerotation_pitch _returnvalue_yaw)) (1000.0 1000.0 1000.0))) :`ObjectTypes` (`|MakeArray` "ObjectTypeQuery1" :!type "EObjectTypeQuery Enum") :`DrawDebugType` "ForDuration")
    (`KismetSystemLibrary.PrintString` "Interacting...")
    (if true
      (`KismetSystemLibrary.PrintString` "Hello"))))

(fn `UserConstructionScript`)