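; Map-design Blueprint that dims the player's flashlight and reveals three special lights in sequence when play begins.
; On BeginPlay it halves the flashlight intensity and narrows its inner cone on the main character.
; It then hides the three SpecialLight references and applies a background material to their cubes.
; One-second delays follow, each turning on the next light's mesh and spotlight and swapping its cube to a light material instance.
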(event `self.ReceiveBeginPlay`
  (bind _speciallightarray (`self.SpecialLightArray`))
  (bind _output (`|GetArrayItem` _speciallightarray 2))
  (bind _output_2 (`|GetArrayItem` _speciallightarray))
  (bind _output_3 (`|GetArrayItem` _speciallightarray 1))
  (bind _asmy_main_character (cast `/Game/Blueprints/CharacterFunctionality/MyMainCharacter` (`GameplayStatics.GetPlayerCharacter` 0)))
  (bind _flashlight (`MainCharacter.Flashlight` _asmy_main_character))
  (`LightComponent.SetIntensity` _flashlight (/ (`LightComponentBase.Intensity` _flashlight) 2.0))
  (`SpotLightComponent.SetInnerConeAngle` _flashlight (/ (`SpotLightComponent.InnerConeAngle` _flashlight) 1.5))
  (set `self.SpecialLightArray` (`|MakeArray` (`self.SpecialLight1`) (`self.SpecialLight2`) (`self.SpecialLight3`)))
  (for _array_element _speciallightarray
    (`SceneComponent.SetVisibility` (`/Game/Blueprints/MapDesign/SpecialLight.LightMesh` _array_element) false false)
    (`SceneComponent.SetVisibility` (`/Game/Blueprints/MapDesign/SpecialLight.SpotLight` _array_element) false false)
    (`PrimitiveComponent.CreateDynamicMaterialInstance` (`/Game/Blueprints/MapDesign/SpecialLight.LightCube` _array_element) 0 "/Engine/EngineMeshes/BackgroundMaterial.BackgroundMaterial" "None"))
  (`KismetSystemLibrary.Delay` 1.0)
  (`SceneComponent.SetVisibility` (`/Game/Blueprints/MapDesign/SpecialLight.LightMesh` _output_2) true false)
  (`SceneComponent.SetVisibility` (`/Game/Blueprints/MapDesign/SpecialLight.SpotLight` _output_2) true false)
  (`PrimitiveComponent.CreateDynamicMaterialInstance` (`/Game/Blueprints/MapDesign/SpecialLight.LightCube` _output_2) 0 "/Game/Materials/LightMaterial.LightMaterial" "None")
  (`KismetSystemLibrary.Delay` 1.0)
  (`SceneComponent.SetVisibility` (`/Game/Blueprints/MapDesign/SpecialLight.LightMesh` _output_3) true false)
  (`SceneComponent.SetVisibility` (`/Game/Blueprints/MapDesign/SpecialLight.SpotLight` _output_3) true false)
  (`PrimitiveComponent.CreateDynamicMaterialInstance` (`/Game/Blueprints/MapDesign/SpecialLight.LightCube` _output_3) 0 "/Game/Materials/LightMaterial.LightMaterial" "None")
  (`KismetSystemLibrary.Delay` 1.0)
  (`SceneComponent.SetVisibility` (`/Game/Blueprints/MapDesign/SpecialLight.LightMesh` _output) true false)
  (`SceneComponent.SetVisibility` (`/Game/Blueprints/MapDesign/SpecialLight.SpotLight` _output) true false)
  (`PrimitiveComponent.CreateDynamicMaterialInstance` (`/Game/Blueprints/MapDesign/SpecialLight.LightCube` _output) 0 "/Game/Materials/LightMaterial.LightMaterial" "None"))

(fn `UserConstructionScript`)